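; Player pawn Blueprint that handles gamepad movement, turn input and keeps the mouse cursor visible every tick.
; Left stick X and Y feed helper functions that add movement along forward and right vectors respectively, built from control pitch only, so yaw does not affect direction.
; The Turn axis adds controller yaw.
; A and D keys set IsLeft and IsRight flags, which nothing here reads.
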(event `Key|A`
  (params (Key :type "Key Structure"))
  (:`Pressed`
    (set `self.isLeft` true))
  (:`Released`
    (set `self.isLeft` false)))

(event `self.ReceiveTick`
  (params (DeltaSeconds :type "Float (single-precision)"))
  ;[1 1 1] move
  (set `PlayerController.bShowMouseCursor` true (`GameplayStatics.GetPlayerController` 0)))

(event `Key|D`
  (params (Key :type "Key Structure"))
  (:`Pressed`
    (set `self.isRight` true))
  (:`Released`
    (set `self.isRight` false)))

(event `Key|S`
  (params (Key :type "Key Structure")))

(event `InputAxisKey|Gamepad_LeftX`
  (params (AxisValue :type "Float (single-precision)"))
  ;[1 1 1] move
  (`self.MovePlayerStickFrontBack` AxisValue))

(event `InputAxis|Turn`
  (params (AxisValue :type "Float (single-precision)"))
  ;[1 1 1] move
  (`self.AddControllerYawInput` AxisValue))

(event `InputAxisKey|Gamepad_LeftY`
  (params (AxisValue :type "Float (single-precision)"))
  ;[1 1 1] move
  (`self.MovePlayerStickLeftRigt` AxisValue))

(fn `MovePlayerStickFrontBack`
  (params (A :type "Float (double-precision)"))
  (`self.AddMovementInput` (`KismetMathLibrary.GetForwardVector` (`KismetMathLibrary.MakeRotator` 0.0 (.pitch (`self.GetControlRotation`)))) A))

(fn `MovePlayerStickLeftRigt`
  (params (A :type "Float (double-precision)"))
  (`self.AddMovementInput` (`KismetMathLibrary.GetRightVector` (`KismetMathLibrary.MakeRotator` 0.0 (.pitch (`self.GetControlRotation`)))) A))

(fn `UserConstructionScript`)